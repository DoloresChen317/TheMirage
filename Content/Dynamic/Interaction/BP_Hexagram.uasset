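; BP_Hexagram is an interaction actor that reveals a Li hexagram and a widget when the player character approaches.
; Both start hidden and become visible when BP_ThirdPersonCharacter begins overlapping the Appearance component, with no logic to hide them again.
; Every tick, LiHexagram rotates to face the player camera, acting as a billboard even while hidden.
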(event `self.ReceiveBeginPlay`
  (`self.ChangeVisibility` false))

(event `self.ReceiveTick`
  (params (DeltaSeconds :type "Float (single-precision)"))
  (`SceneComponent.K2_SetWorldRotation` (`self.LiHexagram`) (`KismetMathLibrary.FindLookAtRotation` (`SceneComponent.K2_GetComponentLocation` (`self.LiHexagram`)) (`SceneComponent.K2_GetComponentLocation` (`PlayerCameraManager.TransformComponent` (`GameplayStatics.GetPlayerCameraManager` 0)))) false false))

(event `ChangeVisibility`
  (params (`Visible?` :type Boolean))
  (`SceneComponent.SetVisibility` (`self.LiHexagram`) `Visible?` false)
  (`SceneComponent.SetVisibility` (`self.Widget`) `Visible?` false))

(event `self.Appearance.OnComponentBeginOverlap`
  (params (OverlappedComponent :type "PrimitiveComponent Object Reference") (OtherActor :type "Actor Object Reference") (OtherComp :type "PrimitiveComponent Object Reference") (OtherBodyIndex :type Integer) (bFromSweep :type Boolean) (SweepResult :type "HitResult Structure (by ref)"))
  (cast `/Game/Dynamic/ThirdPerson/Blueprints/BP_ThirdPersonCharacter` OtherActor)
  (`self.ChangeVisibility` true))

(fn `UserConstructionScript`)