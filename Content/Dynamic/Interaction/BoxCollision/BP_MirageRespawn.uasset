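; BP_MirageRespawn is a mirage-style trigger that relocates whenever the player reaches it.
; When BP_ThirdPersonCharacter overlaps its Box, it spawns a new copy of itself SpawnDistance away from the character in a random horizontal direction, then destroys itself.
; Every Tick, it rotates its TextRender to face the player camera.
; SpawnConeatRandomLocation is an empty stub with unconnected nodes.
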(event `self.ReceiveBeginPlay`)

(event `self.ReceiveTick`
  (params (DeltaSeconds :type "Float (single-precision)"))
  (`SceneComponent.K2_SetWorldRotation` (`self.TextRender`) (`KismetMathLibrary.FindLookAtRotation` (`SceneComponent.K2_GetComponentLocation` (`self.TextRender`)) (`SceneComponent.K2_GetComponentLocation` (`PlayerCameraManager.TransformComponent` (`GameplayStatics.GetPlayerCameraManager` 0)))) false false))

(event `self.Box.OnComponentBeginOverlap`
  (params (OverlappedComponent :type "PrimitiveComponent Object Reference") (OtherActor :type "Actor Object Reference") (OtherComp :type "PrimitiveComponent Object Reference") (OtherBodyIndex :type Integer) (bFromSweep :type Boolean) (SweepResult :type "HitResult Structure (by ref)"))
  (bind _asbp_third_person_character (cast `/Game/Dynamic/ThirdPerson/Blueprints/BP_ThirdPersonCharacter` OtherActor))
  (`|SpawnActorFromClass` "BP_MirageRespawn_C" (`KismetMathLibrary.Conv_VectorToTransform` (+ (`self.K2_GetActorLocation` _asbp_third_person_character) (* (`KismetMathLibrary.GetForwardVector` (`KismetMathLibrary.MakeRotator` 0.0 0.0 (`KismetMathLibrary.RandomFloatInRange` 0.0 360.0))) (`self.SpawnDistance`)))) "Undefined" "MultiplyWithRoot" null null)
  (`self.K2_DestroyActor`))

(fn `SpawnConeatRandomLocation`
  (params (Player :type "/Game/Dynamic/ThirdPerson/Blueprints/BP_ThirdPersonCharacter Object Reference")))

(fn `UserConstructionScript`)